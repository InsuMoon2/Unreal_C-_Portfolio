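; BP_CEnemy_Melee2 is a melee enemy Blueprint that colors its overhead label's health bar by allegiance to the player.
; On BeginPlay it runs the parent logic, then fetches the WB_Label widget from its LabelWidget component and caches player 0 as BP_CPlayer.
; The health fill turns green when team IDs match and red otherwise, evaluated only once at BeginPlay.
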(event `self.ReceiveBeginPlay`
  (`parent.ReceiveBeginPlay`)
  (bind _aswb_label (cast `/Game/_Game/Widget/WB_Label` (`WidgetComponent.GetWidget` (`self.LabelWidget`))))
  (`/Engine/EditorBlueprintResources/StandardMacros.IsValid` _aswb_label
    (:`Is Valid`
      (bind _asbp_cplayer (cast `/Game/_Game/Player/BP_CPlayer` (`GameplayStatics.GetPlayerCharacter` 0)))
      (bind _output_get (set `self.As BP CPlayer` _asbp_cplayer))
      (if (== (`self.GetTeamID` _output_get) (`self.GetTeamID`))
        (bind _health (`/Game/_Game/Widget/WB_Label.Health` _aswb_label))
        (`ProgressBar.SetFillColorAndOpacity` _health (struct :`R` 0.05332 :`G` 1.0 :`A` 1.0))
        (else
          (`ProgressBar.SetFillColorAndOpacity` _health (struct :`R` 1.0 :`A` 1.0)))))))

(fn `UserConstructionScript`)