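; Ground decal actor for Grux's Skill 3 that shows a growing marker, then spawns the skill's follow-up actor.
; On BeginPlay it creates a dynamic material instance for the decal, and a timeline animates that material's Radius parameter.
; When the timeline finishes, it hides the decal, destroys itself and spawns BP_ASkill3_Spawn slightly above its location, owned by OwnerCharacter.
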(event `self.ReceiveBeginPlay`
  (`parent.ReceiveBeginPlay`)
  (bind _returnvalue (`DecalComponent.CreateDynamicMaterialInstance` (`self.Ground_Decal`)))
  (bind _output_get (set `self.MID_Decal` _returnvalue))
  (`DecalComponent.SetDecalMaterial` (`self.Ground_Decal`) _output_get)
  (`self.DecalIncrease`))

(event `self.DecalIncrease`
  (bind (_returnvalue_x _returnvalue_y _returnvalue_z) (`KismetMathLibrary.BreakVector` (`self.K2_GetActorLocation`)))
  (bind (_direction `_새_트랙_0`) (`Timeline|타임라인_0` :!via `PlayFromStart`)
    (:`Update`
      (`MaterialInstanceDynamic.SetScalarParameterValue` (`self.MID_Decal`) "Radius" `_새_트랙_0`))
    (:`Finished`
      (`SceneComponent.SetVisibility` (`self.Ground_Decal`) false false)
      (`self.K2_DestroyActor`)
      (`|SpawnActorFromClass` "/Game/_Game/Weapon/GruxWeapon/Skill/BP_ASkill3_Spawn.BP_ASkill3_Spawn_C" (`KismetMathLibrary.MakeTransform` (`KismetMathLibrary.MakeVector` _returnvalue_x _returnvalue_y (+ _returnvalue_z 15.0)) (struct) (1.0 1.0 1.0)) "Undefined" "OverrideRootScale" (`self.OwnerCharacter`) null))))

(fn `UserConstructionScript`)