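; Weapon attachment Blueprint for dual daggers, managing the socket placement and visibility of the right and left dagger meshes.
; On BeginPlay it calls AttachTo for the right and left spine sockets, then hides both meshes.
; Beginning an equip attaches each mesh to its matching hand socket and shows it.
; Unequipping only hides both meshes, without reattaching them to the spine.
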(event `self.ReceiveBeginPlay`
  (`|ExecutionSequence`
    (:`then_0`
      (`self.AttachTo` "Spine_Dagger_Right")
      (`self.AttachTo` "Spine_Dagger_Left"))
    (:`then_1`
      (`SceneComponent.SetVisibility` (`self.Right_Dagger`) false false)
      (`SceneComponent.SetVisibility` (`self.Left_Dagger`) false false))))

(event `self.OnUnequip`
  (`SceneComponent.SetVisibility` (`self.Left_Dagger`) false false)
  (`SceneComponent.SetVisibility` (`self.Right_Dagger`) false false))

(event `self.OnBeginEquip`
  (`|ExecutionSequence`
    (:`then_0`
      (`self.AttachToMesh` "Hand_Dagger_Right" (`self.Right_Dagger`))
      (`self.AttachToMesh` "Hand_Dagger_Left" (`self.Left_Dagger`)))
    (:`then_1`
      (`SceneComponent.SetVisibility` (`self.Right_Dagger`) true false)
      (`SceneComponent.SetVisibility` (`self.Left_Dagger`) true false))))

(fn `UserConstructionScript`)