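; BP_CAttachment_EnemySword is the sword attachment actor for an enemy, carried on the spine and moved to the hand when equipped.
; BeginPlay and OnUnequip attach it to the Spine_Sword socket, while OnBeginEquip attaches it to Hand_Sword, keeping the Sword component visible in both cases.
; Tick destroys the actor once its owner is no longer valid.
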(event `self.ReceiveBeginPlay`
  (`self.AttachTo` "Spine_Sword" :!label _label)
  (`SceneComponent.SetVisibility` (`self.Sword`) true false))

(event `self.OnUnequip`
  (goto _label))

(event `self.OnBeginEquip`
  (`self.AttachTo` "Hand_Sword")
  (`SceneComponent.SetVisibility` (`self.Sword`) true false))

(event `self.ReceiveTick`
  (params (DeltaSeconds :type "Float (single-precision)"))
  (`parent.ReceiveTick` DeltaSeconds)
  (`/Engine/EditorBlueprintResources/StandardMacros.IsValid` (`self.GetOwner`)
    (:`Is Not Valid`
      (`self.K2_DestroyActor`))))

(fn `UserConstructionScript`)