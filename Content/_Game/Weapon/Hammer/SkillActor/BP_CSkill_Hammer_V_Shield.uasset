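; Skill actor for the Hammer V shield: a configurable sphere with a ground decal and Niagara ground and orb effects.
; The construction script applies size, materials, effect assets and colors, creates the sphere's dynamic material, and sets a slow-mo flag from the Functionality enum.
; On BeginPlay, after the parent logic, it fades in the decal and plays a timeline that drives the material's Appear parameter through a curve.
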(event `self.ReceiveBeginPlay`
  (`parent.ReceiveBeginPlay`)
  (`DecalComponent.SetFadeIn` (`self.Decal`) (`self.DecalFadeDelay`) (`self.DecalFadeDuration`))
  (`TimelineComponent.SetPlayRate` (`self.CirveTick`) (`self.AppearSpeed`))
  (bind (_direction _newtrack_0) (`Timeline|CirveTick`)
    (:`Update`
      (`MaterialInstanceDynamic.SetScalarParameterValue` (`self.InstanceMaterial`) "Appear" (`CurveFloat.GetFloatValue` (`self.AppearCurve`) _newtrack_0)))))

(fn `UserConstructionScript`
  (bind _shield_sphere (`self.Shield_Sphere`))
  (bind _groundvfx (`self.GroundVFX`))
  (bind _orbvfx (`self.OrbVFX`))
  (`|ExecutionSequence`
    (:`then_0`
      (`PrimitiveComponent.SetMaterial` _shield_sphere 0 (`self.ShieldMaterial`))
      (`SceneComponent.SetWorldScale3D` _shield_sphere (`KismetMathLibrary.Conv_DoubleToVector` (`self.ShieldSize`)))
      (bind _returnvalue (`PrimitiveComponent.CreateDynamicMaterialInstance` _shield_sphere 0 null "None"))
      (set `self.InstanceMaterial` _returnvalue))
    (:`then_1`
      (`DecalComponent.SetDecalMaterial` (`self.Decal`) (`self.DecalMaterial`)))
    (:`then_2`
      (switch `/Game/Assets/AdvancedShieldSystem/Blueprints/EnumsAndInterfaces/Enum_ShieldFunction` (`self.Functionality`)
        (:`NewEnumerator2`
          (set `self.IsSlowMo?` false))
        (:`NewEnumerator0`
          (set `self.IsSlowMo?` true))))
    (:`then_3`
      ;[0 0 0 1 20] GroundVFX
      (`FXSystemComponent.SetColorParameter` _groundvfx "User.Color" (`self.GroundVFXColor`))
      (`NiagaraComponent.SetAsset` _groundvfx (`self.GroundEffect`)))
    (:`then_4`
      (`FXSystemComponent.SetColorParameter` _orbvfx "User.Color01" (`self.OrbColor_01`))
      (`FXSystemComponent.SetColorParameter` _orbvfx "User.Color02" (`self.OrbColor_02`))
      (`NiagaraComponent.SetAsset` _orbvfx (`self.OrbParticle`)))))