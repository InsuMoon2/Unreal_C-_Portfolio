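; Bow attachment Blueprint that shows four arrow meshes on the spine of the wielder while the bow is equipped.
; On BeginPlay it attaches each arrow to its own spine_arrow socket through AttachToMesh, then hides all four.
; OnBeginEquip makes the arrows visible and OnUnequip hides them again, each after calling the parent implementation.
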(event `self.ReceiveBeginPlay`
  (`parent.ReceiveBeginPlay`)
  (`|ExecutionSequence`
    (:`then_0`
      (`self.AttachToMesh` "spine_arrow1" (`self.Arrow1`))
      (`self.AttachToMesh` "spine_arrow2" (`self.Arrow2`))
      (`self.AttachToMesh` "spine_arrow3" (`self.Arrow3`))
      (`self.AttachToMesh` "spine_arrow4" (`self.Arrow4`)))
    (:`then_1`
      (`SceneComponent.SetVisibility` (`self.Arrow1`) false false)
      (`SceneComponent.SetVisibility` (`self.Arrow2`) false false)
      (`SceneComponent.SetVisibility` (`self.Arrow3`) false false)
      (`SceneComponent.SetVisibility` (`self.Arrow4`) false false))))

(event `self.OnBeginEquip`
  (`parent.OnBeginEquip`)
  (`|ExecutionSequence`
    (:`then_1`
      (`SceneComponent.SetVisibility` (`self.Arrow1`) true false)
      (`SceneComponent.SetVisibility` (`self.Arrow2`) true false)
      (`SceneComponent.SetVisibility` (`self.Arrow3`) true false)
      (`SceneComponent.SetVisibility` (`self.Arrow4`) true false))))

(event `self.OnUnequip`
  (`parent.OnUnequip`)
  (`SceneComponent.SetVisibility` (`self.Arrow1`) false false)
  (`SceneComponent.SetVisibility` (`self.Arrow2`) false false)
  (`SceneComponent.SetVisibility` (`self.Arrow3`) false false)
  (`SceneComponent.SetVisibility` (`self.Arrow4`) false false))

(fn `UserConstructionScript`)