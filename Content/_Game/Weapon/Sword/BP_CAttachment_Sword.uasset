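; Sword attachment Blueprint that moves the weapon mesh between a holstered socket and a hand socket as it is equipped and unequipped.
; On BeginPlay it attaches to Spine_Sword and shows its skeletal mesh.
; OnBeginEquip moves it to Hand_Sword and makes it visible.
; OnUnequip returns it to Spine_Sword but hides the mesh, unlike its initial visible holstered state.
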(event `self.ReceiveBeginPlay`
  (`self.AttachTo` "Spine_Sword")
  (`SceneComponent.SetVisibility` (`self.SkeletalMesh`) true false))

(event `self.OnUnequip`
  (`self.AttachTo` "Spine_Sword")
  (`SceneComponent.SetVisibility` (`self.SkeletalMesh`) false false))

(event `self.OnBeginEquip`
  (`self.AttachTo` "Hand_Sword")
  (`SceneComponent.SetVisibility` (`self.SkeletalMesh`) true false))

(fn `UserConstructionScript`)