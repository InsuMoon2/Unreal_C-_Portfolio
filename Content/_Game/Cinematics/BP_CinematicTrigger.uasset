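; One-shot trigger volume that plays the Master level sequence as a boss-intro cinematic.
; On overlap it hides top-level widgets, then, inside that same widget loop, starts the sequence, disables player input and collision, and sets a timer.
; When the timer fires it restores widgets except the crosshair, re-enables input, spawns BP_CEnemy_Boss and repositions the player relative to the trigger.
; Both phases unhide Character actors; the trigger finally destroys itself.
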(event `self.Cinematic_Trigger.OnComponentBeginOverlap`
  (params (OverlappedComponent :type "PrimitiveComponent Object Reference") (OtherActor :type "Actor Object Reference") (OtherComp :type "PrimitiveComponent Object Reference") (OtherBodyIndex :type Integer) (bFromSweep :type Boolean) (SweepResult :type "HitResult Structure (by ref)"))
  (bind _foundwidgets (`WidgetBlueprintLibrary.GetAllWidgetsOfClass` "/Script/UMG.UserWidget"))
  (for _array_element _foundwidgets
    (`Widget.SetVisibility` _array_element "Hidden")
    (bind (_outactor _returnvalue) (`LevelSequencePlayer.CreateLevelSequencePlayer` "/Game/_Game/Cinematics/Master.Master"))
    (`MovieSceneSequencePlayer.Play` _returnvalue)
    (`KismetSystemLibrary.K2_SetTimerDelegate` (delegate `CustomEvent`) 14.6)
    (`self.DisableInput` (`GameplayStatics.GetPlayerCharacter` 0) (`GameplayStatics.GetPlayerController` 0))
    (`self.SetActorEnableCollision` false)
    (bind _outactors (`GameplayStatics.GetAllActorsOfClass` "/Script/Engine.Actor"))
    (for _array_element_2 _outactors
      (bind _returnvalue_2 (`GameplayStatics.GetObjectClass` _array_element_2))
      (if (or (`KismetMathLibrary.ClassIsChildOf` _returnvalue_2 "/Script/Engine.Character") (== _returnvalue_2 "/Game/_Game/Widget/WB_HUD.WB_HUD_C"))
        (`self.SetActorHiddenInGame` _array_element_2 false)))))

(event `CustomEvent`
  (bind (_returnvalue_x _returnvalue_y _returnvalue_z) (`KismetMathLibrary.BreakVector` (`self.K2_GetActorLocation`)))
  (bind (_returnvalue_x_2 _returnvalue_y_2 _returnvalue_z_2) (`KismetMathLibrary.BreakVector` (`self.K2_GetActorLocation`)))
  (bind (_returnvalue_roll _returnvalue_pitch _returnvalue_yaw) (`KismetMathLibrary.BreakRotator` (`self.K2_GetActorRotation` (`self.Player`))))
  (bind _foundwidgets (`WidgetBlueprintLibrary.GetAllWidgetsOfClass` "/Script/UMG.UserWidget"))
  (for _array_element _foundwidgets
    (cast `/Game/_Game/Widget/WB_CrossHair` _array_element
      (:`CastFailed`
        (`Widget.SetVisibility` _array_element "Visible")
        (`self.EnableInput` (`GameplayStatics.GetPlayerCharacter` 0) (`GameplayStatics.GetPlayerController` 0)))))
  (`|SpawnActorFromClass` "/Game/_Game/Enemies/Boss/BP_CEnemy_Boss.BP_CEnemy_Boss_C" (`KismetMathLibrary.MakeTransform` (`KismetMathLibrary.MakeVector` (- _returnvalue_x_2 2800.0) _returnvalue_y_2 (- _returnvalue_z_2 120.0))) "Undefined" "OverrideRootScale" (`self.GetOwner`) null)
  (`self.K2_SetActorTransform` (`self.Player`) (`KismetMathLibrary.MakeTransform` (`KismetMathLibrary.MakeVector` (- _returnvalue_x 1600.0) _returnvalue_y (- _returnvalue_z 120.0)) (`KismetMathLibrary.MakeRotator` _returnvalue_roll _returnvalue_pitch _returnvalue_yaw)) false false)
  (bind _outactors (`GameplayStatics.GetAllActorsOfClass` "/Script/Engine.Actor"))
  (for _array_element_2 _outactors
    (bind _returnvalue (`GameplayStatics.GetObjectClass` _array_element_2))
    (if (or (`KismetMathLibrary.ClassIsChildOf` _returnvalue "/Script/Engine.Character") (== _returnvalue "/Game/_Game/Widget/WB_HUD.WB_HUD_C"))
      (`self.SetActorHiddenInGame` _array_element_2 false)))
  (`self.K2_DestroyActor`))

(fn `UserConstructionScript`)